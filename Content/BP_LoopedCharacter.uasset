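; Player character that fights enemies with a short-range forward line-trace attack and returns to the hub level on death.
; Fire deals base damage plus one equipped effect, picked by priority: burn, venom, chain spark, then lifesteal, each enabled by an Activate function.
; Inspect holds a mid-combat slow-mo request through SloMoManager.
; Tick feeds health to the crosshair widget and triggers death, which clears all effects.
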(event `self.ReceiveBeginPlay`
  (set `self.bBurnShotEquipped` false)
  (bind _returnvalue (`|CreateWidget` "/Game/UI/WBP_Crosshair.WBP_Crosshair_C"))
  (`UserWidget.AddToViewport` _returnvalue 0)
  (set `self.CrosshairWidget` _returnvalue))

(event `EnhancedInput|/Game/IA_Inspect`
  (params (ActionValue :type Boolean) (ElapsedSeconds :type "Float (double-precision)") (TriggeredSeconds :type "Float (double-precision)") (InputAction :type "InputAction Object Reference" :default "/Game/IA_Inspect.IA_Inspect"))
  (:`Started`
    (bind _asslo_mo_manager (cast `SloMoManager` (`SubsystemBlueprintLibrary.GetWorldSubsystem` "/Script/Looped.SloMoManager")))
    (`SloMoManager.RequestSloMo` _asslo_mo_manager "MidCombatInspect" 3.0))
  (:`Completed`
    (bind _asslo_mo_manager_2 (cast `SloMoManager` (`SubsystemBlueprintLibrary.GetWorldSubsystem` "/Script/Looped.SloMoManager")))
    (`SloMoManager.ReleaseSloMo` _asslo_mo_manager_2 "MidCombatInspect")))

(event `self.ReceiveTick`
  (params (DeltaSeconds :type "Float (single-precision)"))
  (`self.CrosshairWidget`
    (:`then`
      (`/Game/UI/WBP_Crosshair.SetHP` (`self.CrosshairWidget`) (`self.GetPOCHealthPercent`))
      (if (<= (`self.POCCurrentHealth`) 0.0)
        (`self.HandleDeath`)))
    (:`else`)))

(event `EnhancedInput|/Game/IA_Fire`
  (params (ActionValue :type Boolean) (ElapsedSeconds :type "Float (double-precision)") (TriggeredSeconds :type "Float (double-precision)") (InputAction :type "InputAction Object Reference" :default "/Game/IA_Fire.IA_Fire"))
  (bind _returnvalue (`self.K2_GetActorLocation`))
  (:`Started`
    (bind _outhit (`KismetSystemLibrary.LineTraceSingle` _returnvalue (+ _returnvalue (* (`self.GetActorForwardVector`) 200.0)) "TraceTypeQuery1"))
    (bind _asenemy_base (cast `EnemyBase` (`.HitActor` (`GameplayStatics.BreakHitResult` _outhit))))
    (`EnemyBase.TakeDamageFromPlayer` _asenemy_base 20.0 null)
    (if (`self.bBurnShotEquipped`)
      (`EnemyBase.ApplyBurnEffect` _asenemy_base 10.0 3)
      (elif (`self.bVenomEquipped`)
        (`EnemyBase.ApplyVenomEffect` _asenemy_base 5.0 5 0.4)
        (elif (`self.bChainSparkEquipped`)
          (`EnemyBase.ApplyChainSparkEffect` _asenemy_base 10.0 500.0)
          (elif (`self.bLifestealEquipped`)
            (`EnemyBase.ApplyLifestealEffect` _asenemy_base 5.0)))))))

(fn `ActivateBurnShot`
  (set `self.bBurnShotEquipped` true))

(fn `ActivateChainSpark`
  (set `self.bChainSparkEquipped` true))

(fn `ActivateLifesteal`
  (set `self.bLifestealEquipped` true))

(fn `ActivateVenomShot`
  (set `self.bVenomEquipped` true))

(fn `HandleDeath`
  (set `self.bBurnShotEquipped` false)
  (set `self.bVenomEquipped` false)
  (set `self.bChainSparkEquipped` false)
  (set `self.bLifestealEquipped` false)
  (`GameplayStatics.OpenLevel` "L_Hub"))

(fn `UpdatePlayerHPBar`)

(fn `UserConstructionScript`)