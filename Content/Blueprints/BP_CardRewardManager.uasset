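; Card reward manager that offers passive card picks as enemies are cleared and moves the run to the next room.
; Counts enemies down through the game mode's OnRoomCleared event, then shows WBP_CardReward with independently randomized eligible cards, slow motion and a character hologram.
; A pick equips the card, raises its perk level and resets the count, then travels after enough picks or optionally respawns enemies.
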(event `self.ReceiveBeginPlay`
  (bind _aslooped_run_game_mode (cast `LoopedRunGameMode` (`GameplayStatics.GetGameMode`)))
  (add `LoopedRunGameMode.OnRoomCleared` _aslooped_run_game_mode (delegate `OnRoomClearedCallback`))
  (bind _outactors (`GameplayStatics.GetAllActorsOfClass` "/Script/Looped.EnemyBase"))
  (set `self.EnemiesRemaining` (`KismetArrayLibrary.Array_Length` _outactors)))

(event `OnRoomClearedCallback`
  (bind _output_get (set `self.EnemiesRemaining` (- (`self.EnemiesRemaining`) 1)))
  (if (== _output_get 0)
    (`self.TriggerCardReward`)))

(event `OnCardChosenCallback`
  (bind _returnvalue (`Controller.K2_GetPawn` (`GameplayStatics.GetPlayerController` 0)))
  (bind _aswbp_card_reward (cast `/Game/UI/WBP_CardReward` (`self.CardRewardWidgetRef`))
    (:`then`
      (bind _aspassive_stack_component (cast `PassiveStackComponent` (`self.GetComponentByClass` _returnvalue "/Script/Looped.PassiveStackComponent"))
        (:`then`
          (bind _selectedrowname (`/Game/UI/WBP_CardReward.SelectedRowName` _aswbp_card_reward))
          (`PassiveStackComponent.EquipCard` _aspassive_stack_component _selectedrowname (`PassiveStackComponent.GetFirstEmptySlot` _aspassive_stack_component)))
        (:`CastFailed`
          _)))
    (:`CastFailed`
      _))
  (`Widget.RemoveFromParent` _aswbp_card_reward)
  (bind _aslooped_character (cast `LoopedCharacter` (`GameplayStatics.GetPlayerCharacter` 0)))
  (`LoopedCharacter.CloseHologram` _aslooped_character)
  (bind _asslo_mo_manager (cast `SloMoManager` (`SubsystemBlueprintLibrary.GetWorldSubsystem` "/Script/Looped.SloMoManager")))
  (`SloMoManager.ReleaseSloMo` _asslo_mo_manager "CardSelection")
  (`WidgetBlueprintLibrary.SetInputMode_GameOnly` (`GameplayStatics.GetPlayerController` 0))
  (set `self.CardRewardWidgetRef` null)
  (bind _asbp_looped_character (cast `/Game/BP_LoopedCharacter` _returnvalue))
  (`LoopedCharacter.IncrementPerkLevel` _asbp_looped_character _selectedrowname)
  (set `self.EnemiesRemaining` 3)
  (bind _aslooped_run_game_mode (cast `LoopedRunGameMode` (`GameplayStatics.GetGameMode`)))
  (`LoopedRunGameMode.SetCursorVisibility` _aslooped_run_game_mode false)
  (bind _output_get (set `self.CardPickCount` (+ (`self.CardPickCount`) 1)))
  (if (>= _output_get (`self.PortalAfterPicks`))
    (bind _aslooped_game_instance (cast `LoopedGameInstance` (`GameplayStatics.GetGameInstance`)))
    (`LoopedGameInstance.TravelToNextRoom` _aslooped_game_instance)
    (elif (`self.bEnemiesRespawn`)
      (`LoopedRunGameMode.RespawnAllEnemies` _aslooped_run_game_mode))))

(fn `SelectCardByKey`
  (params (CardIndex :type Integer)))

(fn `TriggerCardReward`
  (bind _workingcards (`self.WorkingCards`))
  (bind _outitem (`KismetArrayLibrary.Array_Random` _workingcards))
  (bind _outitem_2 (`KismetArrayLibrary.Array_Random` _workingcards))
  (bind _outitem_3 (`KismetArrayLibrary.Array_Random` _workingcards))
  (bind _asbp_looped_character (cast `/Game/BP_LoopedCharacter` (`GameplayStatics.GetPlayerCharacter` 0)))
  (set `self.WorkingCards` (`LoopedCharacter.GetEligibleCards` _asbp_looped_character (`self.WorkingCards`)))
  (`DataTableFunctionLibrary.GetDataTableRowNames` (`self.PassiveCardTableRef`))
  (bind _returnvalue (`WidgetBlueprintLibrary.Create` "/Game/UI/WBP_CardReward.WBP_CardReward_C"))
  (bind _aswbp_card_reward (cast `/Game/UI/WBP_CardReward` _returnvalue))
  (`/Game/UI/WBP_CardReward.SetCardOptions` _aswbp_card_reward _outitem_2 _outitem_3 _outitem)
  (bind _aslooped_game_instance (cast `LoopedGameInstance` (`GameplayStatics.GetGameInstance`)))
  (`/Game/UI/WBP_CardReward.ConfigureExtra` _aswbp_card_reward (`LoopedGameInstance.GetCardChoiceCount` _aslooped_game_instance) (`KismetArrayLibrary.Array_Random` (`self.WorkingCards`)))
  (bind _aslooped_character (cast `LoopedCharacter` (`GameplayStatics.GetPlayerCharacter` 0)))
  (`LoopedCharacter.OpenHologramForReward` _aslooped_character)
  (`UserWidget.AddToViewport` _aswbp_card_reward 250)
  (add `/Game/UI/WBP_CardReward.OnCardChosen` _aswbp_card_reward (`|CreateDelegate` :!event `OnCardChosenCallback`))
  (bind _asslo_mo_manager (cast `SloMoManager` (`SubsystemBlueprintLibrary.GetWorldSubsystem` "/Script/Looped.SloMoManager")))
  (`SloMoManager.RequestSloMo` _asslo_mo_manager "CardSelection" 0.0)
  (`WidgetBlueprintLibrary.SetInputMode_GameAndUIEx` (`GameplayStatics.GetPlayerController` 0) null "DoNotLock" false)
  (set `self.CardRewardWidgetRef` _aswbp_card_reward)
  (set `self.ChosenCard1` _outitem_2)
  (set `self.ChosenCard2` _outitem_3)
  (set `self.ChosenCard3` _outitem)
  (bind _aslooped_run_game_mode (cast `LoopedRunGameMode` (`GameplayStatics.GetGameMode`)))
  (`LoopedRunGameMode.SetCursorVisibility` _aslooped_run_game_mode true))

(fn `UserConstructionScript`)